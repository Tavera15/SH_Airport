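; BP_Spawner_A is a one-shot timed spawner that brings an AI NPC in at the player character's location.
; One to two minutes after BeginPlay, it saves the first ThirdPersonCharacter's location, spawns a herb item there and plays a 2D sound.
; Seconds later it spawns an NPC running NPC_BT there, then sets it as MyPawn on the first found NPC's AI controller.
; The SpawnNPC function is empty.
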(event EventBeginPlay
  (Utilities|FlowControl|Delay (Math|Random|RandomFloatinRange 6e+01 1.2e+02))
  (bind _outactors (Actor|GetAllActorsOfClass "/Game/ThirdPersonCPP/Blueprints/ThirdPersonCharacter.ThirdPersonCharacter_C"))
  (bind _output_get (Variables|Default|SetNPCSpawnLocation (.location (Transformation|GetActorTransform (Utilities|Array|Get(acopy) _outactors)))))
  (Game|SpawnActorfromClass "/Game/InventorySystem/Item/Item_A_BP_Herb.Item_A_BP_Herb_C" (Math|Transform|MakeTransform _output_get (.rotation (Transformation|GetActorTransform (Utilities|Array|Get(acopy) _outactors))) "1,1,1") "Undefined" 0 0)
  (Audio|PlaySound2D "/Game/The-Undisputed-Era-_AudioTrimmer_com_-_1_.The-Undisputed-Era-_AudioTrimmer_com_-_1_" 1.0 1.0 0.0 0 0)
  (Utilities|FlowControl|Delay 7.0)
  (bind _returnvalue (AI|SpawnAIFromClass "/Game/NPC/NPC.NPC_C" "/Game/NPC/NPC_BT.NPC_BT" (Variables|Default|GetNPCSpawnLocation) (.rotation (Transformation|GetActorTransform (Utilities|Array|Get(acopy) _outactors))) true))
  (bind _asnpc (Utilities|Casting|CastToNPC _returnvalue))
  (bind _outactors_2 (Actor|GetAllActorsOfClass "/Game/NPC/NPC.NPC_C"))
  (bind _asnpc_aicontroller (Utilities|Casting|CastToNPC_AIController (AI|GetAIController (Utilities|Array|Get(acopy) _outactors_2))))
  (Variables|/Game/NPC/NPC_AIController.NPC_AIController_C|SetMyPawn _asnpc_aicontroller _asnpc))

(fn ConstructionScript)

(fn SpawnNPC)