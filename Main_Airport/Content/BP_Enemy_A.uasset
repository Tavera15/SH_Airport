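; BP_Enemy_A is an enemy actor with a health pool that can be damaged and that hurts the player on contact.
; Point damage subtracts from Health, prints the new value, and destroys the actor once Health reaches zero or below.
; On overlap with a ThirdPersonCharacter, it directly reduces that character's Health by a fixed amount rather than going through the damage system.
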(event EventBeginPlay)

(event Collision|EventActorBeginOverlap
  (params (OtherActor :type Actor%20Object%20Reference))
  (bind _asthird_person_character (Utilities|Casting|CastToThirdPersonCharacter OtherActor))
  (Variables|/Script/Main_Airport.Main_AirportCharacter|SetHealth _asthird_person_character (- (Variables|/Script/Main_Airport.Main_AirportCharacter|GetHealth _asthird_person_character) 2e+01)))

(event EventTick
  (params (DeltaSeconds :type Float%20%28single-precision%29)))

(event Game|Damage|EventPointDamage
  (params (Damage :type Float%20%28single-precision%29) (DamageType :type Damage%20Type%20Object%20Reference) (HitLocation :type Vector :default "0, 0, 0") (HitNormal :type Vector :default "0, 0, 0") (HitComponent :type Primitive%20Component%20Object%20Reference) (BoneName :type Name :default "None") (ShotFromDirection :type Vector :default "0, 0, 0") (InstigatedBy :type Controller%20Object%20Reference) (DamageCauser :type Actor%20Object%20Reference) (HitInfo :type Hit%20Result%20Structure%20%28by%20ref%29))
  (bind _output_get (Variables|Default|SetHealth (- (Variables|Default|GetHealth) Damage)))
  (Development|PrintText (Utilities|Text|ToText(Float) _output_get "HalfToEven"))
  (if (<= _output_get 0.0)
    (Actor|DestroyActor)))

(fn ConstructionScript)