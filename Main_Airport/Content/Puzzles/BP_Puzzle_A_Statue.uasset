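; Puzzle A statue Blueprint that delivers the puzzle's reward when its OnEventReward event fires.
; The event finds the first Key_BP_SecretArtRoom actor in the level and moves it to a hardcoded world location.
; It then spawns a FountainWater_P emitter at a second fixed position near the key.
; The file holds only this reward response, with no puzzle-solving logic of its own.
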(event EventBeginPlay
  (|CallParentFunction) ; This node is disabled and will not be called.\nDrag off pins to build functionality.
)

(event Collision|EventActorBeginOverlap
  (params (OtherActor :type Actor%20Object%20Reference))
  (|CallParentFunction OtherActor) ; This node is disabled and will not be called.\nDrag off pins to build functionality.
)

(event EventTick
  (params (DeltaSeconds :type Float%20%28single-precision%29))
  (|CallParentFunction DeltaSeconds) ; This node is disabled and will not be called.\nDrag off pins to build functionality.
)

(event EventOnEventReward
  (bind _outactors (Actor|GetAllActorsOfClass "/Game/InventorySystem/Item/PuzzleKeys/Key_BP_SecretArtRoom.Key_BP_SecretArtRoom_C"))
  (Transformation|SetActorLocation (Utilities|Array|Get(acopy) _outactors) "-30987.000000,-11900.000000,299.000000" false false)
  (Effects|SpawnEmitteratLocation "/Game/Imported_Items/FountainWater_P.FountainWater_P" "-30727.000000,-11893.000000,546.000000" "0,180.000000, 0"))

(fn ConstructionScript
  (|CallParentFunction))